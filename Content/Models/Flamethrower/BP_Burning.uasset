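; Burnable actor for the flamethrower that, once ignited, burns away and adds to the game score.
; An inactive Niagara voxel flame is attached to its static mesh, and a dynamic overlay material starts invisible.
; Ignite fires once, makes the player drop their item, starts audio and scales up the flames.
; Blazing then animates overlay opacity on a timeline paced by BurnTime before destroying the actor and scoring.
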(event `self.ReceiveBeginPlay`
  (bind _output_get (set `self.Mesh` (`self.GetComponentByClass` "/Script/Engine.StaticMeshComponent")))
  (bind _returnvalue (`NiagaraFunctionLibrary.SpawnSystemAttached` "/Game/Models/Flamethrower/VFX_VoxelFlame_System.VFX_VoxelFlame_System" _output_get "None" (0.0 0.0 0.0) (struct) "KeepRelativeOffset" false false))
  (bind _output_get_2 (set `self.Particles` _returnvalue))
  (`NiagaraFunctionLibrary.OverrideSystemUserVariableStaticMeshComponent` _output_get_2 "" (`self.Mesh`)))

(event `Ignite`
  (bind _particles (`self.Particles`))
  (if (not (`self.IsIgnited`))
    (set `self.IsIgnited` true)
    (bind _asbp_first_person_character (cast `/Game/FirstPerson/Blueprints/BP_FirstPersonCharacter` (`GameplayStatics.GetPlayerCharacter` 0)))
    (`/Game/FirstPerson/Blueprints/BP_FirstPersonCharacter.DropItem` _asbp_first_person_character)
    (`ActorComponent.Activate` _particles false)
    (`AddComponent|NODE_AddAudioComponent-1`)
    (bind (_direction _newtrack_0) (`Timeline|Ignite_Time`)
      (:`Update`
        (`SceneComponent.SetWorldScale3D` _particles (`KismetMathLibrary.MakeVector` _newtrack_0 _newtrack_0 _newtrack_0)))
      (:`Finished`
        (`self.Blazing`)))))

(event `Blazing`
  (set `self.IsBurning` true)
  (`TimelineComponent.SetPlayRate` (`self.Blazing_Time`) (/ 1.0 (`self.BurnTime`)))
  (`AddComponent|NODE_AddAudioComponent-2`)
  (bind (_direction _newtrack_0) (`Timeline|Blazing_Time`)
    (:`Update`
      (`MaterialInstanceDynamic.SetScalarParameterValue` (`self.BurnOverlay`) "Opacity" _newtrack_0))
    (:`Finished`
      (set `self.IsBurning` false)
      (`self.K2_DestroyActor`)
      (set `self.IsIgnited` false)
      (bind _asgm_game_state (cast `/Game/FirstPerson/Blueprints/GM_GameState` (`GameplayStatics.GetGameMode`)))
      (`/Game/FirstPerson/Blueprints/GM_GameState.AddScore` _asgm_game_state))))

(fn `UserConstructionScript`
  (bind _returnvalue (`KismetMaterialLibrary.CreateDynamicMaterialInstance` "/Game/Models/Flamethrower/Overlay_Burning.Overlay_Burning"))
  (bind _output_get (set `self.BurnOverlay` _returnvalue))
  (`MeshComponent.SetOverlayMaterial` (`self.Mesh`) _output_get)
  (`MaterialInstanceDynamic.SetScalarParameterValue` (`self.BurnOverlay`) "Opacity" 0.0))