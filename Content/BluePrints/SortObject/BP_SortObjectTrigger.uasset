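; BP_SortObjectTrigger is a drop spot for objects tagged Sortable in the sorting task.
; On overlap, it snaps the object to the root's relative transform, stops its physics, adds to the GM_GameState score, makes the player drop it and plays a sound.
; Tick shows the Pointer while the player holds a sortable and IsTriggered is true.
; Any overlap clears IsTriggered, even without the tag; SnapPlace is not called here.
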(event `self.Box.OnComponentBeginOverlap`
  (params (OverlappedComponent :type "PrimitiveComponent Object Reference") (OtherActor :type "Actor Object Reference") (OtherComp :type "PrimitiveComponent Object Reference") (OtherBodyIndex :type Integer) (bFromSweep :type Boolean) (SweepResult :type "HitResult Structure (by ref)"))
  (bind _returnvalue (`self.GetComponentByClass` OtherActor "/Script/Engine.PrimitiveComponent"))
  (bind _defaultsceneroot (`self.DefaultSceneRoot`))
  ; Trigger Box
  (set `self.IsTriggered` false)
  (if (`self.ActorHasTag` OtherActor "Sortable")
    (`SceneComponent.K2_SetRelativeLocationAndRotation` _returnvalue (`SceneComponent.RelativeLocation` _defaultsceneroot) (`SceneComponent.RelativeRotation` _defaultsceneroot) false false)
    (`PrimitiveComponent.SetSimulatePhysics` _returnvalue false)
    (bind _asgm_game_state (cast `/Game/BluePrints/GameManager/GM_GameState` (`GameplayStatics.GetGameMode`)))
    (`/Game/BluePrints/GameManager/GM_GameState.AddSortScore_1` _asgm_game_state)
    (bind _asbp_first_person_character (cast `/Game/FirstPerson/Blueprints/BP_FirstPersonCharacter` (`GameplayStatics.GetPlayerCharacter` 0)))
    (if true
      (`/Game/FirstPerson/Blueprints/BP_FirstPersonCharacter.DropItem` _asbp_first_person_character)
      (`GameplayStatics.PlaySound2D` "/Game/sounds/objects/MS_place_object.MS_place_object" 1.0 1.0 0.0 null null))))

(event `self.ReceiveTick`
  (params (DeltaSeconds :type "Float (single-precision)"))
  (bind _pointer (`self.Pointer`))
  ; Sort Pointer
  (bind _returnvalue (`GameplayStatics.GetActorOfClass` "/Game/FirstPerson/Blueprints/BP_FirstPersonCharacter.BP_FirstPersonCharacter_C"))
  (if (and (and (`/Game/FirstPerson/Blueprints/BP_FirstPersonCharacter.HoldingObject` _returnvalue) (`self.IsTriggered`)) (`/Game/FirstPerson/Blueprints/BP_FirstPersonCharacter.HoldSortable` _returnvalue))
    (`SceneComponent.SetVisibility` _pointer true false)
    (`ActorComponent.SetComponentTickEnabled` _pointer true)
    (else
      (`SceneComponent.SetVisibility` _pointer false false)
      (`ActorComponent.SetComponentTickEnabled` _pointer false))))

(event `self.ReceiveBeginPlay`
  ; Sort Pointer
  (set `self.IsTriggered` true))

(fn `SnapPlace`
  (params (NewParam :type "Actor Object Reference") (NewParam1 :type "Actor Object Reference"))
  (if (`self.ActorHasTag` NewParam1 "Interactable")
    (`self.K2_SetActorLocation` NewParam1 (`self.K2_GetActorLocation` NewParam1) false true)
    (`self.K2_SetActorRotation` :`self` NewParam :`bTeleportPhysics` true)
    (`PrimitiveComponent.SetSimulatePhysics` (`self.GetComponentByClass` "/Script/Engine.PrimitiveComponent") false)))

(fn `UserConstructionScript`)