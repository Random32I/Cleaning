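; GM_GameState is the game manager tracking junk score and sort score for a level, with overridable targets.
; BeginPlay derives maximums from BP_Junk and "Trigger"-tagged actor counts, then creates WBP_UI, which the score events update.
; Tick feeds the character's LookAtTag to the toggleable hints and, once both targets are met, clears GameOver and reveals the completion text.
; CompleteLevel then can show the end screen and block movement.
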(event `self.ReceiveBeginPlay`
  (bind _overridescoremax (`self.OverrideScoreMax`))
  (bind _ovveridesortmax (`self.OvverideSortMax`))
  (`WidgetBlueprintLibrary.SetInputMode_GameOnly` (`GameplayStatics.GetPlayerController` 0))
  (`|ExecutionSequence`
    (:`then_0`
      (bind _outactors (`GameplayStatics.GetAllActorsOfClass` "/Game/BluePrints/JunkBP/BP_Junk.BP_Junk_C"))
      (if (== _overridescoremax 0)
        (set `self.MaxScore` (`KismetArrayLibrary.Array_Length` _outactors))
        (else
          (set `self.MaxScore` _overridescoremax))))
    (:`then_1`
      (bind _outactors_2 (`GameplayStatics.GetAllActorsWithTag` "Trigger"))
      (if (== _ovveridesortmax 0)
        (set `self.MaxSortScore` (`KismetArrayLibrary.Array_Length` _outactors_2))
        (else
          (set `self.MaxSortScore` _ovveridesortmax)))
      (bind _returnvalue (`|CreateWidget` "/Game/UI/WBP_UI.WBP_UI_C"))
      (bind _output_get (set `self.UserInterface` _returnvalue))
      (`UserWidget.AddToViewport` _output_get 0)
      (`/Game/UI/WBP_UI.UpdateScore` _output_get 0 (`self.MaxScore`))
      (`/Game/UI/WBP_UI.UpdateSortScore` _output_get 0 (`self.MaxSortScore`)))))

(event `self.ReceiveTick`
  (params (DeltaSeconds :type "Float (single-precision)"))
  (bind _userinterface (`self.UserInterface`))
  ; If Current score = Max score
  (`|ExecutionSequence`
    (:`then_0`
      (if (and (`self.GameOver`) (and (>= (`self.CurrentScore`) (`self.MaxScore`)) (>= (`self.SortScore`) (`self.MaxSortScore`))))
        (set `self.GameOver` false)
        (set `Widget.Visibility` "Visible" (`/Game/UI/WBP_UI.CompleteText` (stale `self.ReceiveBeginPlay` _returnvalue)))))
    (:`then_1`
      (bind _asbp_first_person_character (cast `/Game/FirstPerson/Blueprints/BP_FirstPersonCharacter` (`GameplayStatics.GetPlayerCharacter` 0)))
      (`/Game/UI/WBP_UI.HintGiver` _userinterface (`/Game/FirstPerson/Blueprints/BP_FirstPersonCharacter.LookAtTag` _asbp_first_person_character) (`/Game/UI/WBP_UI.GivingHints` _userinterface)))))

(event `AddScore`
  (bind _currentscore (`self.CurrentScore`))
  (bind _maxscore (`self.MaxScore`))
  ; Add Score by Calling Widget
  (bind _result (`/Engine/EditorBlueprintResources/StandardMacros.IncrementInt` _currentscore)
    (:`  `
      (set `self.ScorePercent` (/ (`KismetMathLibrary.Conv_IntToDouble` _currentscore) (`KismetMathLibrary.Conv_IntToDouble` _maxscore)))
      (`/Game/UI/WBP_UI.UpdateScore` (`self.UserInterface`) _result _maxscore))))

(event `CompleteLevel`
  (bind _returnvalue (`GameplayStatics.GetPlayerController` 0))
  ; Shows End Screen
  (if (not (`self.GameOver`))
    (bind _returnvalue_2 (`|CreateWidget` "/Game/UI/WBP_EndScreen.WBP_EndScreen_C"))
    (`UserWidget.AddToViewport` _returnvalue_2 0)
    (`WidgetBlueprintLibrary.SetInputMode_UIOnlyEx` _returnvalue _returnvalue_2)
    (set `PlayerController.bShowMouseCursor` true _returnvalue)
    (`Controller.SetIgnoreMoveInput` _returnvalue true)))

(event `AddSortScore_1`
  (bind _sortscore (`self.SortScore`))
  (bind _maxsortscore (`self.MaxSortScore`))
  ; Add Sort Score by Calling Widget
  (bind _result (`/Engine/EditorBlueprintResources/StandardMacros.IncrementInt` _sortscore)
    (:`  `
      (set `self.SortPercent` (/ (`KismetMathLibrary.Conv_IntToDouble` _sortscore) (`KismetMathLibrary.Conv_IntToDouble` _maxsortscore)))
      (`/Game/UI/WBP_UI.UpdateSortScore` (`self.UserInterface`) _result _maxsortscore))))

(event `ToggleHint`
  (bind _userinterface (`self.UserInterface`))
  (set `/Game/UI/WBP_UI.GivingHints` (not (`/Game/UI/WBP_UI.GivingHints` _userinterface)) _userinterface))

(fn `AddSortScore`)

(fn `UserConstructionScript`)