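; BP_Junk is a physics-simulated junk prop that can catch fire and spread it to other BP_Burning actors.
; On BeginPlay it enables physics on its primitive component, sets a custom depth stencil and attaches a hidden, scaled sphere fitted to the mesh bounds.
; Sphere begin-overlaps ignite the junk from burning actors, or ignite unlit ones when it burns.
; An older polling check for geometry collection overlaps is left disconnected.
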(event `self.ReceiveBeginPlay`
  (bind _self_sphere (`self.Self_Sphere`))
  (bind _self_sphere_2 (`self.Self_Sphere`))
  (bind _self_mesh (`self.Self_Mesh`))
  ; Set Physics and Custom Depth
  (bind _output_get (set `self.Self_Mesh` (`self.GetComponentByClass` "/Script/Engine.PrimitiveComponent")))
  (`parent.ReceiveBeginPlay`)
  (`PrimitiveComponent.SetSimulatePhysics` _output_get true)
  (`PrimitiveComponent.SetCustomDepthStencilValue` _output_get 2)
  ; Sets Sphere Collider for Burning
  (bind _returnvalue (`AddComponent|NODE_AddSphereComponent-0`))
  (bind _output_get_2 (set `self.Self_Sphere` _returnvalue))
  (`SceneComponent.SetHiddenInGame` _output_get_2 true false)
  (`SceneComponent.K2_AttachToComponent` _self_sphere _self_mesh "None" "KeepRelative" "KeepRelative" "KeepRelative" true)
  (`SceneComponent.K2_SetWorldLocation` _self_sphere (`PrimitiveComponent.GetCenterOfMass` _self_mesh "None") false false)
  (`SphereComponent.SetSphereRadius` _self_sphere (`.SphereRadius` (`KismetSystemLibrary.GetComponentBounds` _self_mesh)) true)
  (`SceneComponent.SetRelativeScale3D` _self_sphere_2 (`KismetMathLibrary.Conv_DoubleToVector` (`self.CollideScaleSphere`)))
  (add `PrimitiveComponent.OnComponentBeginOverlap` _self_sphere_2 (delegate `SphereOverlapBegin`)))

(event `self.ReceiveActorBeginOverlap`
  (params (OtherActor :type "Actor Object Reference"))
  (`parent.ReceiveActorBeginOverlap` null))

(event `SphereOverlapBegin`
  (params (OverlappedComponent :type "PrimitiveComponent Object Reference") (OtherActor :type "Actor Object Reference") (OtherComp :type "PrimitiveComponent Object Reference") (OtherBodyIndex :type Integer) (bFromSweep :type Boolean) (SweepResult :type "HitResult Structure (by ref)"))
  ; Burning Overlap
  (`|ExecutionSequence`
    (:`then_0`
      (bind _output_get (set `self.Other Actor` OtherActor))
      (if (not (== _output_get (`self.Self_Sphere`)))
        (bind _asbp_burning (cast `/Game/BluePrints/Burning/BP_Burning` (`self.Other Actor`)))
        (if (`/Game/BluePrints/Burning/BP_Burning.IsBurning` _asbp_burning)
          (if (not (`self.IsBurning`))
            (`self.Ignite`)))))
    (:`then_1`
      (if (`self.IsBurning`)
        (bind _output_get_2 (set `self.Other Actor` OtherActor))
        (if (not (== _output_get_2 (`self.Self_Sphere`)))
          (bind _asbp_burning_2 (cast `/Game/BluePrints/Burning/BP_Burning` (`self.Other Actor`)))
          (if (not (`/Game/BluePrints/Burning/BP_Burning.IsBurning` _asbp_burning_2))
            (`self.Ignite` _asbp_burning_2)))))))

(event `self.ReceiveTick`
  (params (DeltaSeconds :type "Float (single-precision)"))
  ; Constant Burn Check (Disabled)
  (`parent.ReceiveTick` 0.0))

(fn `UserConstructionScript`
  (`parent.UserConstructionScript`))