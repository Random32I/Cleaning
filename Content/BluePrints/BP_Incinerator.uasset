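; BP_Incinerator is an actor that burns Interactable objects that hit it, ignoring those tagged Junk.
; A valid hit makes the player drop the held item, increments the UI's ObjectsBurned count, destroys the object, adds an audio component and awards score through GM_GameState.
; A parallel sequence branch activates a Niagara effect for two seconds.
; An unconnected level-load check is left in the graph and never runs.
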(event `self.ReceiveHit`
  (params (MyComp :type "PrimitiveComponent Object Reference") (Other :type "Actor Object Reference") (OtherComp :type "PrimitiveComponent Object Reference") (bSelfMoved :type Boolean) (HitLocation :type "Vector Structure") (HitNormal :type "Vector Structure") (NormalImpulse :type "Vector Structure") (Hit :type "HitResult Structure (by ref)"))
  (bind _niagara (`self.Niagara`))
  (if (`self.ActorHasTag` Other "Junk")
    _
    (elif (`self.ActorHasTag` Other "Interactable")
      (`|ExecutionSequence`
        (:`then_0`
          (bind _asbp_first_person_character (cast `/Game/FirstPerson/Blueprints/BP_FirstPersonCharacter` (`GameplayStatics.GetPlayerCharacter` 0)))
          (`/Game/FirstPerson/Blueprints/BP_FirstPersonCharacter.DropItem` _asbp_first_person_character)
          (bind _uiwidget (`/Game/FirstPerson/Blueprints/BP_FirstPersonCharacter.UIWidget` _asbp_first_person_character))
          (set `/Game/FirstPerson/Blueprints/HUD.ObjectsBurned` (+ (`/Game/FirstPerson/Blueprints/HUD.ObjectsBurned` _uiwidget) 1) _uiwidget)
          (`self.K2_DestroyActor` Other)
          (`AddComponent|NODE_AddAudioComponent-0`)
          (bind _asgm_game_state (cast `/Game/FirstPerson/Blueprints/GM_GameState` (`GameplayStatics.GetGameMode`)))
          (`/Game/FirstPerson/Blueprints/GM_GameState.AddScore` _asgm_game_state))
        (:`then_1`
          (`ActorComponent.Activate` _niagara false)
          (`KismetSystemLibrary.Delay` 2.0)
          (`ActorComponent.Deactivate` _niagara))))))

(fn `UserConstructionScript`)