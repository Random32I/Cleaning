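; BP_JunkBreakMix is a breakable physics junk object that shatters into pieces.
; On BeginPlay it enables physics simulation on its primitive component and sets that component's custom depth stencil value.
; Its Breaking function plays a 2D break sound, destroys the actor, then spawns each class in NumBreakPieces at the supplied location and rotation.
; Breaking has no caller within this Blueprint.
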(event `self.ReceiveBeginPlay`
  (bind _returnvalue (`self.GetComponentByClass` "/Script/Engine.PrimitiveComponent"))
  (`parent.ReceiveBeginPlay`)
  (`PrimitiveComponent.SetSimulatePhysics` _returnvalue true)
  (`PrimitiveComponent.SetCustomDepthStencilValue` _returnvalue 4))

(event `self.ReceiveActorBeginOverlap`
  (params (OtherActor :type "Actor Object Reference"))
  (`parent.ReceiveActorBeginOverlap` null))

(event `self.ReceiveTick`
  (params (DeltaSeconds :type "Float (single-precision)"))
  (`parent.ReceiveTick` 0.0))

(fn `Breaking`
  (params (ObjectLocation :type "Vector Structure") (ObjectRotation :type "Rotator Structure"))
  (`GameplayStatics.PlaySound2D` "/Game/sounds/objects/MS_break.MS_break" 1.0 1.0 0.0 null null)
  (`self.K2_DestroyActor`)
  (for _array_element (`self.numBreakPieces`)
    (`|SpawnActorFromClass` _array_element (`KismetMathLibrary.MakeTransform` ObjectLocation ObjectRotation) "Undefined" "MultiplyWithRoot" null null)))

(fn `UserConstructionScript`
  (`parent.UserConstructionScript`))