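; BP_BreakObject is a breakable physics prop that is replaced by pieces when broken.
; On BeginPlay it enables physics simulation on its primitive component and sets that component's custom depth stencil value.
; Breaking destroys the actor, then spawns every class in the NumBreakPieces array at the supplied location.
; Nothing in this Blueprint calls Breaking, and its random scatter offset nodes are left unconnected.
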(event `self.ReceiveBeginPlay`
  (bind _returnvalue (`self.GetComponentByClass` "/Script/Engine.PrimitiveComponent"))
  (`PrimitiveComponent.SetSimulatePhysics` _returnvalue true)
  (`PrimitiveComponent.SetCustomDepthStencilValue` _returnvalue 4))

(fn `Breaking`
  (params (ObjectLocation :type "Vector Structure"))
  (`self.K2_DestroyActor`)
  (for _array_element (`self.numBreakPieces`)
    (`|SpawnActorFromClass` _array_element (`KismetMathLibrary.Conv_VectorToTransform` ObjectLocation) "Undefined" "MultiplyWithRoot" null null)))

(fn `UserConstructionScript`)